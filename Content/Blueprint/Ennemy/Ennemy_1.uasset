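; Enemy character that chases the player, switching between projectile fire and parryable melee attacks.
; Overlap volumes set speed and attack mode; Tick drives Delay-timed strikes and line-trace-gated shots using the Blackboard's FollowPlayer flag.
; At low HP it moves and attacks faster, takes half damage and counts melee hits received.
; On death it releases the player's lock-on and may drop ammo or heal rewards, based on that count and a random roll.
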(event `self.ReceiveBeginPlay`
  ;[1 1 1] Event begin play
  ;;[1 1 1] Get player actor reference
  (bind _outactors (`GameplayStatics.GetAllActorsOfClass` "/Game/Player/Player.Player_C"))
  (set `self.PlayerReference` (`|GetArrayItem` _outactors)))

(event `/Game/Blueprint/Interface/Modificator.TakeDamage`
  (params (AmountOfDamage :type Integer) (From :type String))
  ;[1 1 1] Take damage
  (if (`self.LowHP`)
    ;;[1 1 1] If lowHP
    (switch `string` From
      (:`Projectile`
        _)
      (:`CaC`
        (`/Engine/EditorBlueprintResources/StandardMacros.IncrementInt` (`self.NumberOfAttackCacTake`)
          (:`  `
            _))))
    (set `self.Life` (- (`self.Life`) (/ AmountOfDamage 2)))
    (else
      (bind _output_get (set `self.Life` (- (`self.Life`) AmountOfDamage)))
      (if (<= _output_get 10)
        (set `self.LowHP` true)
        (set `CharacterMovementComponent.MaxWalkSpeed` 700.0 (`self.CharacterMovement`))))))

(event `self.CaCAttack.OnComponentBeginOverlap`
  (params (OverlappedComponent :type "PrimitiveComponent Object Reference") (OtherActor :type "Actor Object Reference") (OtherComp :type "PrimitiveComponent Object Reference") (OtherBodyIndex :type Integer) (bFromSweep :type Boolean) (SweepResult :type "HitResult Structure (by ref)"))
  (bind _charactermovement (`self.CharacterMovement`))
  ;[1 1 1] Only CaC attack detection
  (cast `/Game/Player/Player` OtherActor)
  (set `self.CaC_AttackOnly` true)
  (if (`BlackboardComponent.GetValueAsBool` (`AIBlueprintHelperLibrary.GetBlackboard` self) "FollowPlayer")
    (if (`self.LowHP`)
      (set `CharacterMovementComponent.MaxWalkSpeed` 900.0 _charactermovement)
      (else
        (set `CharacterMovementComponent.MaxWalkSpeed` 800.0 _charactermovement)))))

(event `self.CaCAttack.OnComponentEndOverlap`
  (params (OverlappedComponent :type "PrimitiveComponent Object Reference") (OtherActor :type "Actor Object Reference") (OtherComp :type "PrimitiveComponent Object Reference") (OtherBodyIndex :type Integer))
  (bind _charactermovement (`self.CharacterMovement`))
  ;[1 1 1] Only CaC attack detection
  (cast `/Game/Player/Player` OtherActor)
  (set `self.CaC_AttackOnly` false)
  (if (`self.LowHP`)
    (set `CharacterMovementComponent.MaxWalkSpeed` 600.0 _charactermovement)
    (else
      (set `CharacterMovementComponent.MaxWalkSpeed` 400.0 _charactermovement))))

(event `self.ReceiveTick`
  (params (DeltaSeconds :type "Float (single-precision)"))
  (bind _returnvalue (`self.GetControlRotation`))
  (bind _capsulecomponent (`self.CapsuleComponent`))
  (bind _playerreference (`self.PlayerReference`))
  (bind _numberofattackcactake (`self.NumberOfAttackCacTake`))
  (bind _returnvalue_2 (`SceneComponent.K2_GetComponentLocation` _capsulecomponent))
  (bind _returnvalue_3 (`SceneComponent.K2_GetComponentToWorld` (`self.CapsuleComponent`)))
  (`|ExecutionSequence`
    (:`then_0`
      ;[1 1 1] Life display
      (`/Engine/EditorBlueprintResources/StandardMacros.IsValid` (`self.PlayerReference`)
        (:`Is Valid`
          ;;[1 1 1] Set text life for player
          (`TextRenderComponent.K2_SetText` (`self.LifeTextDisplay`) (`KismetTextLibrary.Conv_IntToText` (`self.Life`))))))
    (:`then_1`
      ;[1 1 1] Destroy if the life as 0
      (if (<= (`self.Life`) 0)
        ;;[1 1 1] Reset camera if ennemy is lock
        (if (`self.isTarget`)
          (`/Game/Player/Player.Set-Reset camera CaC` _playerreference)
          (`/Game/Player/Player.ResetLockTarget` _playerreference))
        (switch `int` (`KismetMathLibrary.RandomIntegerInRange` 0 2)
          (:`0`
            (if (>= _numberofattackcactake 3)
              (`|SpawnActorFromClass` "/Game/Blueprint/AmmoReward.AmmoReward_C" _returnvalue_3 "Undefined" "OverrideRootScale" null null))
            (`self.K2_DestroyActor`))
          (:`1`
            (if (>= _numberofattackcactake 5)
              (`|SpawnActorFromClass` "/Game/Blueprint/HealReward.HealReward_C" _returnvalue_3 "Undefined" "OverrideRootScale" null null))
            (`self.K2_DestroyActor`))
          (:`2`
            (if (>= _numberofattackcactake 5)
              (`|SpawnActorFromClass` "/Game/Blueprint/AmmoReward.AmmoReward_C" _returnvalue_3 "Undefined" "OverrideRootScale" null null)
              (`|SpawnActorFromClass` "/Game/Blueprint/HealReward.HealReward_C" _returnvalue_3 "Undefined" "OverrideRootScale" null null))
            (`self.K2_DestroyActor`)))))
    (:`then_2`
      ;[1 1 1] Attack system
      (if (`self.CanAttack`)
        (bind _asplayer (cast `/Game/Player/Player` (`GameplayStatics.GetPlayerCharacter` 0)))
        (bind (_parrystruct_canparry _parrystruct_isparry) (break `/Game/Blueprint/Structure/ParryStructure` (`/Game/Player/Player.ParryStruct` _asplayer)))
        (set `/Game/Player/Player.ParryStruct` (make `/Game/Blueprint/Structure/ParryStructure` true _parrystruct_isparry) _asplayer)
        (if (`self.LowHP`)
          (`KismetSystemLibrary.Delay` "1f")
          (else
            (`KismetSystemLibrary.Delay` "1.5f")))
        (message `/Game/Blueprint/Interface/Modificator.ResetCombo` (`GameplayStatics.GetPlayerCharacter` 0))
        (if (`self.CanAttack`)
          (bind _asplayer_2 (cast `/Game/Player/Player` (`GameplayStatics.GetPlayerCharacter` 0)))
          (bind (_parrystruct_canparry_2 _parrystruct_isparry_2) (break `/Game/Blueprint/Structure/ParryStructure` (`/Game/Player/Player.ParryStruct` _asplayer_2)))
          (if _parrystruct_isparry_2
            (bind _asplayer_3 (cast `/Game/Player/Player` (`GameplayStatics.GetPlayerCharacter` 0)))
            (bind _parrystruct_canparry_3 (break `/Game/Blueprint/Structure/ParryStructure` (`/Game/Player/Player.ParryStruct` _asplayer_3)))
            (set `/Game/Player/Player.ParryStruct` (make `/Game/Blueprint/Structure/ParryStructure` _parrystruct_canparry_3) _asplayer_3)
            (else
              (bind _asplayer_4 (cast `/Game/Player/Player` (`GameplayStatics.GetPlayerPawn` 0)))
              (`/Game/Player/Player.TakeDamage` _asplayer_4 10 "CaC")
              (bind _parrystruct_canparry_4 (break `/Game/Blueprint/Structure/ParryStructure` (`/Game/Player/Player.ParryStruct` _asplayer_4)))
              (set `/Game/Player/Player.ParryStruct` (make `/Game/Blueprint/Structure/ParryStructure` _parrystruct_canparry_4) _asplayer_4))))))
    (:`then_3`
      ;[1 1 1] Shooting system
      (`/Engine/EditorBlueprintResources/StandardMacros.IsValid` self
        (:`Is Valid`
          (if (and (not (`self.CanAttack`)) (`BlackboardComponent.GetValueAsBool` (`AIBlueprintHelperLibrary.GetBlackboard` self) "FollowPlayer") (not (`self.CaC_AttackOnly`)))
            (bind _outhit (`KismetSystemLibrary.LineTraceSingle` :`Start` _returnvalue_2 :`End` (+ _returnvalue_2 (* (`KismetMathLibrary.GetForwardVector` (`SceneComponent.K2_GetComponentRotation` _capsulecomponent)) "5000f")) :`TraceChannel` "TraceTypeQuery1" :`DrawDebugType` "ForOneFrame"))
            (cast `/Game/Player/Player` (`.HitActor` (`GameplayStatics.BreakHitResult` _outhit)))
            (if (`self.LowHP`)
              (`KismetSystemLibrary.Delay` "0.25f")
              (else
                (`KismetSystemLibrary.Delay` "0.5f")))
            (`|SpawnActorFromClass` "/Game/Blueprint/Ennemy/E_Projectile.E_Projectile_C" (`KismetMathLibrary.MakeTransform` (+ (`self.K2_GetActorLocation`) (* (`KismetMathLibrary.GetForwardVector` _returnvalue) "100f")) _returnvalue) "Undefined" "OverrideRootScale" null null)))))))

(event `self.AttackPlayer.OnComponentBeginOverlap`
  (params (OverlappedComponent :type "PrimitiveComponent Object Reference") (OtherActor :type "Actor Object Reference") (OtherComp :type "PrimitiveComponent Object Reference") (OtherBodyIndex :type Integer) (bFromSweep :type Boolean) (SweepResult :type "HitResult Structure (by ref)"))
  ;[1 1 1] Can / can't attack player
  (cast `/Game/Player/Player` OtherActor)
  (set `self.CanAttack` true)
  (bind _asplayer (cast `/Game/Player/Player` (`GameplayStatics.GetPlayerCharacter` 0)))
  (bind (_cacstruct_isoncac _cacstruct_isoncombo _cacstruct_combo _cacstruct_damage _cacstruct_comboorder _cacstruct_refactualactor) (break `/Game/Blueprint/Structure/CacStructure` (`/Game/Player/Player.CacStruct` _asplayer)))
  (set `/Game/Player/Player.CacStruct` (make `/Game/Blueprint/Structure/CacStructure` true false _cacstruct_combo _cacstruct_damage _cacstruct_comboorder _cacstruct_refactualactor) _asplayer)
  (`/Game/Player/Player.Set-Reset camera CaC` (`self.PlayerReference`)))

(event `self.AttackPlayer.OnComponentEndOverlap`
  (params (OverlappedComponent :type "PrimitiveComponent Object Reference") (OtherActor :type "Actor Object Reference") (OtherComp :type "PrimitiveComponent Object Reference") (OtherBodyIndex :type Integer))
  ;[1 1 1] Can / can't attack player
  (cast `/Game/Player/Player` OtherActor)
  (set `self.CanAttack` false)
  (bind _asplayer (cast `/Game/Player/Player` (`GameplayStatics.GetPlayerCharacter` 0)))
  (set `/Game/Player/Player.ParryStruct` (make `/Game/Blueprint/Structure/ParryStructure` false) _asplayer)
  (bind (_cacstruct_isoncac _cacstruct_isoncombo _cacstruct_combo _cacstruct_damage _cacstruct_comboorder _cacstruct_refactualactor) (break `/Game/Blueprint/Structure/CacStructure` (`/Game/Player/Player.CacStruct` _asplayer)))
  (set `/Game/Player/Player.CacStruct` (make `/Game/Blueprint/Structure/CacStructure` false false _cacstruct_combo _cacstruct_damage _cacstruct_comboorder _cacstruct_refactualactor) _asplayer)
  (`/Game/Player/Player.Set-Reset camera CaC` (`self.PlayerReference`)))

(event `/Game/Blueprint/Interface/Modificator.SetVisibilityInTarget`
  ;[1 1 1] Set visibility on target
  (bind _isa (`/Engine/EditorBlueprintResources/StandardMacros.FlipFlop`)
    (:`A`
      _)
    (:`B`
      _))
  (bind _output_get (set `self.isTarget` _isa))
  (`SceneComponent.SetVisibility` (`self.TargetPoint`) _output_get false))

(fn `UserConstructionScript`)