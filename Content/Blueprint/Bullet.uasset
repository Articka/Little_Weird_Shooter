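; Bullet projectile actor that damages players and Ennemy_1 enemies on hit and destroys itself two seconds after spawning.
; Its sphere hit event identifies the target by class display-name prefix, then casts and calls TakeDamage.
; Enemy hits also set the WasShoot and FollowPlayer blackboard flags to alert the AI.
; Hits on other bullets are ignored, while other unmatched actors such as environment destroy the bullet.
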(event `self.ReceiveBeginPlay`
  ;[1 1 1] Destroy actor after 5 seconds of existance :'(
  (`KismetSystemLibrary.Delay` "2f")
  (`self.K2_DestroyActor`))

(event `self.Sphere.OnComponentHit`
  (params (HitComponent :type "PrimitiveComponent Object Reference") (OtherActor :type "Actor Object Reference") (OtherComp :type "PrimitiveComponent Object Reference") (NormalImpulse :type "Vector Structure") (Hit :type "HitResult Structure (by ref)"))
  (bind _returnvalue (`AIBlueprintHelperLibrary.GetBlackboard` OtherActor))
  (bind _returnvalue_2 (`KismetSystemLibrary.GetClassDisplayName` (`GameplayStatics.GetObjectClass` OtherActor)))
  ;[1 1 1] When bullet hit
  ;[1 1 1] For detect Ennemy_x
  (switch `string` (`KismetStringLibrary.GetSubstring` _returnvalue_2 0 8)
    (:`Default`
      ;[1 1 1] For detect player
      (if (`KismetStringLibrary.EqualEqual_StrStr` (`KismetStringLibrary.GetSubstring` _returnvalue_2 0 6) "Player")
        (bind _asplayer (cast `/Game/Player/Player` OtherActor))
        (`/Game/Player/Player.TakeDamage` _asplayer 10 "Projectile")
        (`self.K2_DestroyActor`)
        (else
          (cast `/Game/Blueprint/Bullet` OtherActor
            (:`CastFailed`
              ;[1 1 1] For other (environment etc.)
              (`self.K2_DestroyActor`))))))
    (:`Ennemy_1`
      (bind _asennemy_1 (cast `/Game/Blueprint/Ennemy/Ennemy_1` OtherActor))
      (`/Game/Blueprint/Ennemy/Ennemy_1.TakeDamage` _asennemy_1 10 "Projectile")
      ;;[1 1 1] AI
      (`BlackboardComponent.SetValueAsBool` _returnvalue "WasShoot" true)
      (`BlackboardComponent.SetValueAsBool` _returnvalue "FollowPlayer" true)
      (`self.K2_DestroyActor`))))

(fn `UserConstructionScript`)